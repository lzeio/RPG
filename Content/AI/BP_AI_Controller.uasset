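; AI controller that runs the BT_AI behavior tree and feeds its blackboard from AI perception updates.
; Each update passes to both sight and hearing handlers, which filter by sense class.
; A successful sight sets Target Actor, while lost sight or any non-sight stimulus, including hearing, clears it.
; A successful hearing stimulus writes its location to InvestigationLocation.
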(event `self.ReceiveBeginPlay`
  (`self.RunBehaviorTree` "/Game/AI/BT_AI.BT_AI"))

(event `self.AIPerception.OnTargetPerceptionUpdated`
  (params (Actor :type "Actor Object Reference") (Stimulus :type "AIStimulus Structure"))
  ;[0.05098 0.05098 0.05098] Set Insight Target
  (`self.HandleSight` Stimulus Actor)
  (`self.HandleHearing` Stimulus Actor))

(fn `HandleHearing`
  (params (Stimulus :type "AIStimulus Structure") (Actor :type "Object Object Reference"))
  (bind (_age _expirationage _strength _stimuluslocation _receiverlocation _tag _bsuccessfullysensed) (break `AIStimulus` Stimulus))
  (bind _returnvalue (`AIPerceptionSystem.GetSenseClassForStimulus` Stimulus))
  (if (== _returnvalue "/Script/AIModule.AISense_Hearing")
    (if _bsuccessfullysensed
      (`BlackboardComponent.SetValueAsVector` (`AIBlueprintHelperLibrary.GetBlackboard` null) "InvestigationLocation" _stimuluslocation))))

(fn `HandleSight`
  (params (Stimulus :type "AIStimulus Structure (by ref)") (Actor :type "Object Object Reference"))
  (bind _returnvalue (`AIBlueprintHelperLibrary.GetBlackboard` null))
  (bind _returnvalue_2 (`AIPerceptionSystem.GetSenseClassForStimulus` Stimulus))
  (if (== _returnvalue_2 "/Script/AIModule.AISense_Sight")
    (if (`.bSuccessfullySensed` (break `AIStimulus` Stimulus))
      (`BlackboardComponent.SetValueAsObject` _returnvalue "Target Actor" Actor)
      (else
        (`BlackboardComponent.ClearValue` _returnvalue "Target Actor" :!label _label)))
    (else
      (goto _label))))

(fn `UserConstructionScript`)
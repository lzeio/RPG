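; Attack system component that handles sword attack input and combo flow, apparently work in progress.
; IA_Attack triggers SwordAttack when CanAttack is set, which either buffers the press during an attack or switches on AttackIndex.
; SwordAttackCombo consumes the buffered press to re-enter that switch, otherwise StopCombo resets the state.
; The switch outputs are empty, montage playback is unconnected, and a separate Attack1 event advances the index through a DoOnce and delay.
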(event `Attack 1`
  ;[0.05098 0.05098 0.05098] Attack 1
  (`/Engine/EditorBlueprintResources/StandardMacros.DoOnce` false :!label _label
    (:`Completed`
      (`KismetSystemLibrary.Delay` 0.1)
      (set `self.Attack Index` 1)
      (goto _label :!via `Reset`))))

(event `EnhancedInput|/Game/ThirdPerson/Input/Actions/IA_Attack`
  (params (ActionValue :type Boolean) (ElapsedSeconds :type "Float (double-precision)") (TriggeredSeconds :type "Float (double-precision)") (InputAction :type "InputAction Object Reference" :default "/Game/ThirdPerson/Input/Actions/IA_Attack.IA_Attack"))
  ;[0.05098 0.05098 0.05098] Attack Input
  (:`Started`
    (if (`self.Can Attack`)
      (`self.Sword Attack`))))

(event `Sword Attack`
  ;[0.05098 0.05098 0.05098] Sword Attack
  (if (`self.Is Attacking`)
    (set `self.Save Attack` true)
    (else
      (set `self.Save Attack` false)
      (switch `int` (`self.Attack Index`) :!label _label_2))))

(event `Sword Attack Combo`
  ;[0.05098 0.05098 0.05098] Sword Combo
  (if (`self.Save Attack`)
    (set `self.Save Attack` false)
    (goto _label_2)
    (else
      (`self.Stop Combo`))))

(event `Stop Combo`
  ;[0.05098 0.05098 0.05098] Stop Attack
  (set `self.Is Attacking` false)
  (set `self.Attack Index` 0))
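; Player stats component for BP_ThirdPersonCharacter that tracks health, stamina, XP and level.
; A tick after BeginPlay it caches the owning character and fills the HUD, which each change function then updates directly.
; Decrease functions report depletion, and reaching max XP triggers a single level-up that carries over surplus XP and raises the threshold.
; Max boosts refill their stat, though the stamina boost builds on current rather than max stamina.
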(event `self.ReceiveBeginPlay`
  (`KismetSystemLibrary.DelayUntilNextTick`)
  (bind _asbp_third_person_character (cast `/Game/ThirdPerson/Blueprints/BP_ThirdPersonCharacter` (`self.GetOwner`)))
  (set `self.Third Person Character BP` _asbp_third_person_character)
  (`ProgressBar.SetPercent` (`/Game/UI/WB_HUD.StaminaBar` (`/Game/ThirdPerson/Blueprints/BP_ThirdPersonCharacter.HUD Widget` (`self.Third Person Character BP`))) (/ (`self.Current Stamina`) (`self.Max Stamina`)))
  (`ProgressBar.SetPercent` (`/Game/UI/WB_HUD.HealthBar` (`/Game/ThirdPerson/Blueprints/BP_ThirdPersonCharacter.HUD Widget` (`self.Third Person Character BP`))) (/ (`self.Current Health`) (`self.Max Health`)))
  (`ProgressBar.SetPercent` (`/Game/UI/WB_HUD.XPMeter` (`/Game/ThirdPerson/Blueprints/BP_ThirdPersonCharacter.HUD Widget` (`self.Third Person Character BP`))) (/ (`self.XP`) (`self.Max XP`)))
  (`TextBlock.SetText` (`/Game/UI/WB_HUD.XPCount` (`/Game/ThirdPerson/Blueprints/BP_ThirdPersonCharacter.HUD Widget` (`self.Third Person Character BP`))) (`|FormatText` "{Current XP} / {Max XP}" (`self.XP`) (`self.Max XP`)))
  (`TextBlock.SetText` (`/Game/UI/WB_HUD.LevelIndex` (`/Game/ThirdPerson/Blueprints/BP_ThirdPersonCharacter.HUD Widget` (`self.Third Person Character BP`))) (`KismetTextLibrary.Conv_IntToText` (`self.Level`))))

(fn `Decrease Health`
  (params (Damage :type "Float (double-precision)"))
  (returns (`Is Player Dead` :type Boolean))
  (bind _current_health (`self.Current Health`))
  (bind _output_get (set `self.Current Health` (`KismetMathLibrary.FClamp` (- _current_health Damage) 0.0 _current_health)))
  (`ProgressBar.SetPercent` (`/Game/UI/WB_HUD.HealthBar` (`/Game/ThirdPerson/Blueprints/BP_ThirdPersonCharacter.HUD Widget` (`self.Third Person Character BP`))) (/ _output_get (`self.Max Health`)))
  (if (<= (`self.Current Health`) 0.0)
    (return true)
    (else
      (return false))))

(fn `Decrease Stamina`
  (params (Fatigue :type "Float (double-precision)"))
  (returns (`Stamina Depleted` :type Boolean))
  (bind _current_stamina (`self.Current Stamina`))
  (bind _output_get (set `self.Current Stamina` (`KismetMathLibrary.FClamp` (- _current_stamina Fatigue) 0.0 _current_stamina)))
  (`ProgressBar.SetPercent` (`/Game/UI/WB_HUD.StaminaBar` (`/Game/ThirdPerson/Blueprints/BP_ThirdPersonCharacter.HUD Widget` (`self.Third Person Character BP`))) (/ _output_get (`self.Max Stamina`)))
  (if (<= _output_get 0.0)
    (return true)
    (else
      (return false))))

(fn `Increase Health`
  (params (`Health Gained` :type "Float (double-precision)"))
  (bind _output_get (set `self.Current Health` (`KismetMathLibrary.FClamp` (+ `Health Gained` (`self.Current Health`)) 0.0 (`self.Max Health`))))
  (`ProgressBar.SetPercent` (`/Game/UI/WB_HUD.HealthBar` (`/Game/ThirdPerson/Blueprints/BP_ThirdPersonCharacter.HUD Widget` (`self.Third Person Character BP`))) (/ _output_get (`self.Max Health`))))

(fn `Increase Level`
  (params (`Added Level` :type Integer))
  (set `self.Level` (+ `Added Level` (`self.Level`)))
  (if (>= (`self.XP`) (`self.Max XP`))
    (set `self.XP` (- (`self.XP`) (`self.Max XP`)))
    (else
      (set `self.XP` 0.0)))
  (set `self.Max XP` (+ (`self.Max XP`) 150.0))
  (`TextBlock.SetText` (`/Game/UI/WB_HUD.LevelIndex` (`/Game/ThirdPerson/Blueprints/BP_ThirdPersonCharacter.HUD Widget` (`self.Third Person Character BP`))) (`KismetTextLibrary.Conv_IntToText` (`self.Level`))))

(fn `Increase Max Health`
  (params (`Health Boost` :type "Float (double-precision)"))
  (bind _output_get (set `self.Max Health` (+ `Health Boost` (`self.Max Health`))))
  (bind _output_get_2 (set `self.Current Health` _output_get))
  (`ProgressBar.SetPercent` (`/Game/UI/WB_HUD.HealthBar` (`/Game/ThirdPerson/Blueprints/BP_ThirdPersonCharacter.HUD Widget` (`self.Third Person Character BP`))) (/ _output_get_2 _output_get)))

(fn `Increase Max Stamina`
  (params (`Stamina Boost` :type "Float (double-precision)"))
  (bind _output_get (set `self.Max Stamina` (+ `Stamina Boost` (`self.Current Stamina`))))
  (set `self.Current Stamina` _output_get)
  (`ProgressBar.SetPercent` (`/Game/UI/WB_HUD.StaminaBar` (`/Game/ThirdPerson/Blueprints/BP_ThirdPersonCharacter.HUD Widget` (`self.Third Person Character BP`))) (/ _output_get (`self.Max Stamina`))))

(fn `Increase Stamina`
  (params (`Stamina Gained` :type "Float (double-precision)"))
  (bind _output_get (set `self.Current Stamina` (`KismetMathLibrary.FClamp` (+ `Stamina Gained` (`self.Current Stamina`)) 0.0 (`self.Max Stamina`))))
  (`ProgressBar.SetPercent` (`/Game/UI/WB_HUD.StaminaBar` (`/Game/ThirdPerson/Blueprints/BP_ThirdPersonCharacter.HUD Widget` (`self.Third Person Character BP`))) (/ _output_get (`self.Max Stamina`))))

(fn `Increase XP`
  (params (B :type "Float (double-precision)"))
  (bind _xp (`self.XP`))
  (set `self.XP` (+ B _xp))
  (if (>= _xp (`self.Max XP`))
    (`self.Increase Level` 1))
  (`ProgressBar.SetPercent` (`/Game/UI/WB_HUD.XPMeter` (`/Game/ThirdPerson/Blueprints/BP_ThirdPersonCharacter.HUD Widget` (`self.Third Person Character BP`))) (/ (`self.XP`) (`self.Max XP`)))
  (`TextBlock.SetText` (`/Game/UI/WB_HUD.XPCount` (`/Game/ThirdPerson/Blueprints/BP_ThirdPersonCharacter.HUD Widget` (`self.Third Person Character BP`))) (`|FormatText` "{Current XP} / {Max XP}" (`self.XP`) (`self.Max XP`))))